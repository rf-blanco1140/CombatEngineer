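; BP_Teammates represents the player's team under fire, with health that drains over time.
; On BeginPlay it creates a team HP widget and starts two self-calling delay loops: steady damage and gunfire/explosion sounds at random intervals.
; When HP runs out, it calls a team-death dispatcher after a short delay and removes the widget.
; The player controller's restart dispatcher resets HP and re-enters the HUD, sound and damage setup.
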(event Custom|DamageTeam
  ;[1 1 1] Team getting damaged over time
  (Variables|Default|SetHP (- (Variables|Default|GetHP) (Variables|Default|GetDamageReceived)))
  (Utilities|FlowControl|Delay (Variables|Default|GetDamageDelay))
  (CallFunction|DamageTeam)
  ;[1 1 1] Teammates Death
  (if (<= (Variables|Default|GetHP) 0)
    (Utilities|FlowControl|Delay 2.0)
    (Default|CallTeamDeathDispatcher)
    (Widget|RemovefromParent (Variables|Default|GetHP_HUD))))

(event Custom|OnLevel%20Restart
  ;[1 1 1] Subscribe and execute the Game Restart Dispatcher
  (Variables|Default|SetHP 100)
  ;[1 1 1] Create Team Status HUD
  (bind _returnvalue (UserInterface|CreateWidget "/Game/BPs/Widgets/BP_W_TeamHP.BP_W_TeamHP_C"))
  (bind _output_get (Variables|Default|SetHP_HUD _returnvalue))
  (Variables|/Game/BPs/Widgets/BP_W_TeamHP.BP_W_TeamHP_C|SetTeamObjectRef _output_get self)
  (UserInterface|Viewport|AddtoViewport (Variables|Default|GetHP_HUD) 0)
  ;[1 1 1] Call to Play Shooting Sounds
  (CallFunction|Gunshoots)
  ;[1 1 1] Team getting damaged over time
  (Variables|Default|SetHP (- (Variables|Default|GetHP) (Variables|Default|GetDamageReceived)))
  (Utilities|FlowControl|Delay (Variables|Default|GetDamageDelay))
  (CallFunction|DamageTeam)
  ;[1 1 1] Teammates Death
  (if (<= (Variables|Default|GetHP) 0)
    (Utilities|FlowControl|Delay 2.0)
    (Default|CallTeamDeathDispatcher)
    (Widget|RemovefromParent (Variables|Default|GetHP_HUD))))

(event Custom|Gunshoots
  ;[1 1 1] Plays Gunshot Sounds
  (Audio|PlaySoundatLocation "/Game/Audio/Snd_Team_Explosions_Cue.Snd_Team_Explosions_Cue" (Transformation|GetActorLocation) "0, 0, 0" 0.5 1.0 0.0 0 0 0)
  (Utilities|FlowControl|Delay (Math|Random|RandomFloatinRange (Variables|Default|GetShootingDelay_1) (Variables|Default|GetShootingDelay_2)))
  (CallFunction|Gunshoots))

(event EventBeginPlay
  ;[1 1 1] Subscribe and execute the Game Restart Dispatcher
  (bind _asbp_pc_main_game (Utilities|Casting|CastToBP_PC_MainGame (Game|GetPlayerController 0)))
  (EventDispatchers|BindEventtoRestartGameDispatcher _asbp_pc_main_game (delegate Custom|OnLevel%20Restart))
  ;[1 1 1] Create Team Status HUD
  (bind _returnvalue (UserInterface|CreateWidget "/Game/BPs/Widgets/BP_W_TeamHP.BP_W_TeamHP_C"))
  (bind _output_get (Variables|Default|SetHP_HUD _returnvalue))
  (Variables|/Game/BPs/Widgets/BP_W_TeamHP.BP_W_TeamHP_C|SetTeamObjectRef _output_get self)
  (UserInterface|Viewport|AddtoViewport (Variables|Default|GetHP_HUD) 0)
  ;[1 1 1] Call to Play Shooting Sounds
  (CallFunction|Gunshoots)
  ;[1 1 1] Team getting damaged over time
  (Variables|Default|SetHP (- (Variables|Default|GetHP) (Variables|Default|GetDamageReceived)))
  (Utilities|FlowControl|Delay (Variables|Default|GetDamageDelay))
  (CallFunction|DamageTeam)
  ;[1 1 1] Teammates Death
  (if (<= (Variables|Default|GetHP) 0)
    (Utilities|FlowControl|Delay 2.0)
    (Default|CallTeamDeathDispatcher)
    (Widget|RemovefromParent (Variables|Default|GetHP_HUD))))

(fn ConstructionScript)