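; Enemy turret that sweeps back and forth while idle and fires at the player on sight.
; Tick yaws it by a fixed step, flipping direction each cycle and saving the current rotation.
; PawnSensing snaps it toward player pawn 0 and spawns projectiles on a 1.5-second cooldown unless the player has failed.
; A retriggerable delay restores the saved rotation and resumes sweeping once sightings stop.
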(event OnSeePawn(PawnSensing)
  (params (Pawn :type Pawn%20Object%20Reference))
  ;[1 1 1] Aiming at Player
  (Utilities|FlowControl|Sequence
    (:then_0
      (Variables|Default|SetHasSeenPlayer true)
      (if (not (Variables|Default|GetHasPlayerFailed))
        (if (== Pawn (Game|Player|GetPlayerPawn 0))
          (Utilities|FlowControl|Sequence
            (:then_0
              (Transformation|SetActorRotation (Math|Rotator|FindLookatRotation (Transformation|GetActorLocation) (Transformation|GetActorLocation Pawn))))
            (:then_1
              ;[1 1 1] Shooting at Player
              (if (Variables|Default|GetSpawnProjectile)
                (Game|SpawnActorfromClass "/Game/BPs/BP_EnemyProjectile_Turret.BP_EnemyProjectile_Turret_C" (Transformation|GetWorldTransform (Variables|Default|GetProjectileSpawnLocation)) "Undefined" 0 0)
                (Variables|Default|SetSpawnProjectile false)
                (Utilities|FlowControl|Delay 1.5)
                (Variables|Default|SetSpawnProjectile true)))))))
    (:then_1
      ;[1 1 1] Checks if is Still Detecting the Player
      (Utilities|FlowControl|RetriggerableDelay 0.6)
      (Transformation|SetActorRotation (Variables|Default|GetCurrentRotation))
      (Variables|Default|SetHasSeenPlayer false))))

(event EventTick
  (params (DeltaSeconds :type Float%20%28single-precision%29))
  (bind _returnvalue (Transformation|GetActorRotation))
  (bind _rotationchangevalue (Variables|Default|GetRotationChangeValue))
  ;[1 1 1] Looping Rotation While Player is Hidden
  (if (not (Variables|Default|GetHasSeenPlayer))
    (if (Variables|Default|GetRotatingRight)
      (Transformation|SetActorRelativeRotation (Math|Rotator|MakeRotator (.roll _returnvalue) (.pitch _returnvalue) (- (.yaw _returnvalue) _rotationchangevalue)))
      (else
        (Transformation|SetActorRelativeRotation (Math|Rotator|MakeRotator (.roll _returnvalue) (.pitch _returnvalue) (+ (.yaw _returnvalue) _rotationchangevalue)))))
    (Variables|Default|SetRemaningRotation (- (Variables|Default|GetRemaningRotation) (Variables|Default|GetRotationChangeValue)))
    (if (<= (Variables|Default|GetRemaningRotation) 0.0)
      (bind _isa (Utilities|FlowControl|FlipFlop)
        (:A
          _)
        (:B
          _))
      (Variables|Default|SetRotatingRight _isa)
      (Variables|Default|SetRemaningRotation (Variables|Default|GetRotationCicleValue))
      (Variables|Default|SetCurrentRotation (Transformation|GetActorRotation)))))

(event EventBeginPlay
  ;[1 1 1] Initialize Neutral Rotation Variable
  (Variables|Default|SetNeutralRotation (Transformation|GetActorRotation)))

(fn ConstructionScript
  (|CallParentFunction))