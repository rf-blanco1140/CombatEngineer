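; Metal grid actor that the player can cut through by interacting until it is destroyed.
; Highlight events swap six cube meshes between a pulsing yellow emissive material and steel.
; Interacting adds a progress bar widget linked to the grid, then a recursive half-second delay loop plays a cutting sound and increments progress.
; At 100 the widget and actor are removed; stopping early removes the widget but keeps accumulated progress.
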(event Custom|CheckIfFinished
  ;[1 1 1] Destroy Object
  (if (Variables|Default|GetIsBeingInteracted)
    (if (>= (Variables|Default|GetActionProgress) 100)
      (Widget|RemovefromParent (Variables|Default|GetWidget))
      (Actor|DestroyActor)
      (else
        (Utilities|FlowControl|Delay 0.5)
        (if (Variables|Default|GetIsBeingInteracted)
          (Utilities|IncrementProgress)
          (CallFunction|CheckifFinished))))))

(event EventBeginPlay)

(event Collision|EventActorBeginOverlap
  (params (OtherActor :type Actor%20Object%20Reference)))

(event EventTick
  (params (DeltaSeconds :type Float%20%28single-precision%29)))

(event EventInteractwithObject
  ;[1 1 1] Destroy Object
  (Utilities|AddProgressionBarWidget)
  (Variables|Default|SetIsBeingInteracted true)
  (if (>= (Variables|Default|GetActionProgress) 100)
    (Widget|RemovefromParent (Variables|Default|GetWidget))
    (Actor|DestroyActor)
    (else
      (Utilities|FlowControl|Delay 0.5)
      (if (Variables|Default|GetIsBeingInteracted)
        (Utilities|IncrementProgress)
        (CallFunction|CheckifFinished)))))

(event EventTurnHighlighton
  ;[1 1 1] Turn Highlight ON/OFF
  (Rendering|Material|SetMaterial (Variables|Default|GetCube) 0 "/Game/Materials/M__Inst_PulsingEmissiveObject_Yellow.M__Inst_PulsingEmissiveObject_Yellow")
  (Rendering|Material|SetMaterial (Variables|Default|GetCube1) 0 "/Game/Materials/M__Inst_PulsingEmissiveObject_Yellow.M__Inst_PulsingEmissiveObject_Yellow")
  (Rendering|Material|SetMaterial (Variables|Default|GetCube2) 0 "/Game/Materials/M__Inst_PulsingEmissiveObject_Yellow.M__Inst_PulsingEmissiveObject_Yellow")
  (Rendering|Material|SetMaterial (Variables|Default|GetCube3) 0 "/Game/Materials/M__Inst_PulsingEmissiveObject_Yellow.M__Inst_PulsingEmissiveObject_Yellow")
  (Rendering|Material|SetMaterial (Variables|Default|GetCube4) 0 "/Game/Materials/M__Inst_PulsingEmissiveObject_Yellow.M__Inst_PulsingEmissiveObject_Yellow")
  (Rendering|Material|SetMaterial (Variables|Default|GetCube5) 0 "/Game/Materials/M__Inst_PulsingEmissiveObject_Yellow.M__Inst_PulsingEmissiveObject_Yellow"))

(event EventTurnHighlightOff
  ;[1 1 1] Turn Highlight ON/OFF
  (Rendering|Material|SetMaterial (Variables|Default|GetCube) 0 "/Game/StarterContent/Materials/M_Metal_Steel.M_Metal_Steel")
  (Rendering|Material|SetMaterial (Variables|Default|GetCube1) 0 "/Game/StarterContent/Materials/M_Metal_Steel.M_Metal_Steel")
  (Rendering|Material|SetMaterial (Variables|Default|GetCube2) 0 "/Game/StarterContent/Materials/M_Metal_Steel.M_Metal_Steel")
  (Rendering|Material|SetMaterial (Variables|Default|GetCube3) 0 "/Game/StarterContent/Materials/M_Metal_Steel.M_Metal_Steel")
  (Rendering|Material|SetMaterial (Variables|Default|GetCube4) 0 "/Game/StarterContent/Materials/M_Metal_Steel.M_Metal_Steel")
  (Rendering|Material|SetMaterial (Variables|Default|GetCube5) 0 "/Game/StarterContent/Materials/M_Metal_Steel.M_Metal_Steel"))

(event EventStopInteracting
  ;[1 1 1] Stop Desroying Object
  (Variables|/Game/BPs/Widgets/BP_W_ProgressionBar.BP_W_ProgressionBar_C|SetIsMetalGrid (Variables|Default|GetWidget) false)
  (Variables|Default|SetIsBeingInteracted false)
  (Widget|RemovefromParent (Variables|Default|GetWidget)))

(fn ConstructionScript)

(fn GetProgress
  (return 0))