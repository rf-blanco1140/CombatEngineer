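; Repairable long cover-bag object that swaps a broken mesh for a repaired, collidable one once the player finishes interacting with it.
; Interacting adds a progress bar widget linked to this actor and starts a half-second delay loop that increments progress while interaction continues.
; At 100 progress it removes the widget and marks itself fixed, while stopping early just removes the widget.
; Highlight events swap the broken mesh's material to pulsing yellow and back.
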(event Custom|CheckIfFinished
  (bind _repairedbags (Variables|Default|GetRepairedBags))
  ;[1 1 1] Repair Bags
  (if (>= (Variables|Default|GetActionProgress) 100)
    (Widget|RemovefromParent (Variables|Default|GetWidget))
    (Development|SetHiddeninGame _repairedbags false false)
    (Collision|SetCollisionEnabled _repairedbags "QueryAndPhysics")
    (Development|SetHiddeninGame (Variables|Default|GetBrokenBags) true false)
    (Variables|Default|SetIsFixed true)
    (else
      (Utilities|FlowControl|Delay 0.5)
      (if (Variables|Default|GetIsBeingInteracted)
        (Utilities|IncrementProgress)
        (CallFunction|CheckifFinished)))))

(event EventBeginPlay
  (bind _repairedbags (Variables|Default|GetRepairedBags))
  ;[1 1 1] Hide Repaired Bags Mesh on BeginPlay
  (Development|SetHiddeninGame _repairedbags true false)
  (Collision|SetCollisionEnabled _repairedbags "NoCollision"))

(event EventTurnHighlighton
  ;[1 1 1] Turn Highlights ON/OFF
  (Rendering|Material|SetMaterial (Variables|Default|GetBrokenBags) 0 "/Game/Materials/M__Inst_PulsingEmissiveObject_Yellow.M__Inst_PulsingEmissiveObject_Yellow"))

(event EventTurnHighlightOff
  ;[1 1 1] Turn Highlights ON/OFF
  (Rendering|Material|SetMaterial (Variables|Default|GetBrokenBags) 0 "/Game/StarterContent/Materials/M_Basic_Wall.M_Basic_Wall"))

(event EventInteractwithObject
  (bind _repairedbags (Variables|Default|GetRepairedBags))
  ;[1 1 1] Repair Bags
  (Utilities|AddsProgressionBarWidget)
  (Variables|Default|SetIsBeingInteracted true)
  (if (not (Variables|Default|GetIsFixed))
    (if (>= (Variables|Default|GetActionProgress) 100)
      (Widget|RemovefromParent (Variables|Default|GetWidget))
      (Development|SetHiddeninGame _repairedbags false false)
      (Collision|SetCollisionEnabled _repairedbags "QueryAndPhysics")
      (Development|SetHiddeninGame (Variables|Default|GetBrokenBags) true false)
      (Variables|Default|SetIsFixed true)
      (else
        (Utilities|FlowControl|Delay 0.5)
        (if (Variables|Default|GetIsBeingInteracted)
          (Utilities|IncrementProgress)
          (CallFunction|CheckifFinished))))))

(event EventStopInteracting
  ;[1 1 1] Stop being repaired
  (Variables|/Game/BPs/Widgets/BP_W_ProgressionBar.BP_W_ProgressionBar_C|SetIsCoverWall (Variables|Default|GetWidget) false)
  (Variables|Default|SetIsBeingInteracted false)
  (Widget|RemovefromParent (Variables|Default|GetWidget)))

(fn ConstructionScript)

(fn GetProgress
  (return 0))