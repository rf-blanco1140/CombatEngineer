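; Main-game player controller that owns the player HUD and handles death, restart and victory flow.
; On begin play and each restart, it creates the HUD and binds to player destruction, team death and final-door win events.
; These events set state flags that Confirm reads to open the main menu, teleport the pawn to spawn, or spawn and possess a new character.
; Dispatchers broadcast player death and restarts.
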(event Custom|OnRespawnSetUp
  ;[1 1 1] Creates Player HUD
  (Default|CallRestartGameDispatcher)
  (bind _returnvalue (UserInterface|CreateWidget "/Game/BPs/Widgets/BP_W_PlayerHUD.BP_W_PlayerHUD_C"))
  (bind _output_get (Variables|Default|SetHUD _returnvalue))
  (UserInterface|Viewport|AddtoViewport _output_get 0)
  ;[1 1 1] Bind to Player Character Death Dispatcher
  (bind _asthird_person_character (Utilities|Casting|CastToThirdPersonCharacter (Game|GetPlayerCharacter 0)))
  (Game|BindEventtoOnDestroyed _asthird_person_character (delegate Custom|OnPlayerDeath))
  ;[1 1 1] Binds to the Team Death Dispatcher
  (bind _returnvalue_2 (Actor|GetActorOfClass "/Game/BPs/BP_Teammates.BP_Teammates_C"))
  (EventDispatchers|BindEventtoTeamDeathDispatcher _returnvalue_2 (delegate Custom|OnTeamDeath))
  ;[1 1 1] Subscribe to GameWon Dispatcher
  (bind _returnvalue_3 (Actor|GetActorOfClass "/Game/BPs/BP_FinalDoor.BP_FinalDoor_C"))
  (EventDispatchers|BindEventtoGameWon _returnvalue_3 (delegate Custom|OnGameWon)))

(event Custom|OnPlayerDeath
  (params (DestroyedActor :type Actor%20Object%20Reference))
  ;[1 1 1] Manages Player Death
  (Widget|RemovefromParent (Variables|Default|GetHUD))
  (Utilities|FlowControl|Delay 2.0)
  (Default|CallPlayerDeathDispatcher)
  (Variables|Default|SetIsPlayerDead true))

(event Custom|OnTeamDeath
  ;[1 1 1] Binds to the Team Death Dispatcher
  (Widget|RemovefromParent (Variables|Default|GetHUD))
  (Variables|Default|SetIsTeamDead true))

(event Custom|OnGameWon
  ;[1 1 1] Subscribe to GameWon Dispatcher
  (Utilities|FlowControl|Delay 2.0)
  (Variables|Default|SetGameWon true))

(event EventBeginPlay
  ;[1 1 1] Creates Player HUD
  (bind _returnvalue (UserInterface|CreateWidget "/Game/BPs/Widgets/BP_W_PlayerHUD.BP_W_PlayerHUD_C"))
  (bind _output_get (Variables|Default|SetHUD _returnvalue))
  (UserInterface|Viewport|AddtoViewport _output_get 0)
  ;[1 1 1] Bind to Player Character Death Dispatcher
  (bind _asthird_person_character (Utilities|Casting|CastToThirdPersonCharacter (Game|GetPlayerCharacter 0)))
  (Game|BindEventtoOnDestroyed _asthird_person_character (delegate Custom|OnPlayerDeath))
  ;[1 1 1] Binds to the Team Death Dispatcher
  (bind _returnvalue_2 (Actor|GetActorOfClass "/Game/BPs/BP_Teammates.BP_Teammates_C"))
  (EventDispatchers|BindEventtoTeamDeathDispatcher _returnvalue_2 (delegate Custom|OnTeamDeath))
  ;[1 1 1] Subscribe to GameWon Dispatcher
  (bind _returnvalue_3 (Actor|GetActorOfClass "/Game/BPs/BP_FinalDoor.BP_FinalDoor_C"))
  (EventDispatchers|BindEventtoGameWon _returnvalue_3 (delegate Custom|OnGameWon)))

(event Input|ActionEvents|InputActionConfirm
  (params (Key :type Key%20Structure :default "None"))
  (bind _spawntransform (Variables|Default|GetSpawnTransform))
  ;[1 1 1] Check if game is won to go back to the main menu
  (:Pressed
    (if (Variables|Default|GetGameWon)
      (Game|OpenLevel(byObjectReference) "/Game/Levels/Lv_MainMenu.Lv_MainMenu")
      (else
        ;[1 1 1] Restart Game
        (if (Variables|Default|GetIsTeamDead)
          (bind _asthird_person_character (Utilities|Casting|CastToThirdPersonCharacter (Game|Player|GetPlayerPawn 0)))
          (Transformation|SetActorLocation _asthird_person_character (.location _spawntransform) false false)
          (Transformation|SetActorRotation _asthird_person_character (.rotation _spawntransform))
          (Variables|Default|SetIsTeamDead false)
          (CallFunction|OnRespawnSetUp)
          (elif (Variables|Default|GetIsPlayerDead)
            (bind _returnvalue (Game|SpawnActorfromClass "/Game/BPs/ThirdPersonCharacter.ThirdPersonCharacter_C" (Variables|Default|GetSpawnTransform) "Undefined" 0 0))
            (Pawn|Possess _returnvalue)
            (CallFunction|OnRespawnSetUp)
            (Variables|Default|SetIsPlayerDead false)))))))

(fn ConstructionScript)